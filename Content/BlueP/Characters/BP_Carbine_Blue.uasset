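; BP_Carbine_Blue is a blue-side first-person character with a hitscan attack and a health pool.
; Attack input fires a debug-drawn visibility line trace forward from the camera.
; Hit actors with "Red" in their display name receive fixed damage through a PistolDamage message.
; Its own PistolDamage event subtracts and prints Health, but the zero-health branch is empty.
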(event EventPistolDamage
  (params (Damage :type Integer) (Bone%20HIt :type Name :default "None"))
  ;[1 1 1] Damage
  (Variables|Default|SetHealth (- (Variables|Default|GetHealth) Damage))
  (Development|PrintString (Utilities|String|ToString(Integer) (Variables|Default|GetHealth)))
  (if (<= (Variables|Default|GetHealth) 0)
    _))

(event Input|ActionEvents|InputActionAttack
  (params (Key :type Key%20Structure))
  (bind _firstpersoncamera (Variables|Default|GetFirstPersonCamera))
  (bind _returnvalue (Transformation|GetWorldLocation _firstpersoncamera))
  ;[1 1 1] Pistol Fire
  (:Pressed
    (bind _outhit (Collision|LineTraceByChannel _returnvalue (+ _returnvalue (* (Math|Vector|GetForwardVector _firstpersoncamera) 5e+03)) "TraceTypeQuery1" false 0 "ForDuration"))
    (if (Utilities|String|Contains (Utilities|GetDisplayName (.HitActor (Collision|BreakHitResult _outhit))) "Red" false true)
      (Class|Interfaces|PistolDamage(Message) (.HitActor (Collision|BreakHitResult _outhit)) 10 "None"))))

(fn ConstructionScript)